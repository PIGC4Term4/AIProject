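; Security camera that detects the first-person player through actor overlap and raises an alarm.
; On entry it turns its spotlight red and broadcasts PlayerFound with the first SecuritySpawner_BP's location and rotation.
; A Gate with a Delay loop repeats the broadcast every second while the player stays inside.
; Leaving closes the gate and restores the white light after a short delay.
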(event EventActorBeginOverlap
  (params (OtherActor :type Actor%20Object%20Reference))
  (bind _outactors (Actor|GetAllActorsOfClass "/Game/Blueprints/SecuritySpawner_BP.SecuritySpawner_BP_C"))
  (Utilities|Casting|CastToFirstPersonCharacter OtherActor)
  (Rendering|Components|Light|SetLightColor (Variables|Default|GetSpotLight) "(R=1.000000,G=0.044127,B=0.000000,A=1.000000)" true)
  (Utilities|FlowControl|Sequence
    (:then_0
      (goto _label Open))
    (:then_1
      (Utilities|FlowControl|Gate false :!label _label
        (:Exit
          (Utilities|FlowControl|Sequence
            (:then_0
              (Default|CallPlayerFound (Transformation|GetActorLocation (Utilities|Array|Get(acopy) _outactors)) (Transformation|GetActorRotation (Utilities|Array|Get(acopy) _outactors))))
            (:then_1
              (Utilities|FlowControl|Delay 1.0)
              (goto _label))))))))

(event Collision|EventActorEndOverlap
  (params (OtherActor :type Actor%20Object%20Reference))
  (Utilities|Casting|CastToFirstPersonCharacter OtherActor)
  (Utilities|FlowControl|Sequence
    (:then_0
      (Utilities|FlowControl|Gate false) ; enters at Close
    )
    (:then_1
      (Utilities|FlowControl|Delay 0.2)
      (Rendering|Components|Light|SetLightColor (Variables|Default|GetSpotLight) "(R=1.000000,G=1.000000,B=1.000000,A=1.000000)" true))))

(fn ConstructionScript)